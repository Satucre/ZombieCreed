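; GameManager_BP is a wave manager for a zombie game, starting the first wave check on BeginPlay.
; When no zombies remain, CheckForNextWave increments the wave and derives both zombie count and spawn weight budget from wave number and ZombieMultiplier.
; ChooseZombies, uncalled here, queues random ZombiWeigth keys using time-seeded streams.
; It draws the weight separately and assigns its negation to the budget instead of subtracting.
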(event EventBeginPlay
  (CallFunction|CheckforNextWave))

(event Collision|EventActorBeginOverlap
  (params (OtherActor :type Actor%20Object%20Reference)))

(event EventTick
  (params (DeltaSeconds :type Float%20%28single-precision%29)))

(fn ConstructionScript)

(fn GetWeightforWave
  (params (Wave :type Integer))
  (return (* (+ Wave (Variables|Default|GetZombieMultiplier)) 2)))

(fn CheckforNextWave
  (if (== (Variables|Default|GetZombieLeftInWave) 0)
    (bind _result (Math|Integer|IncrementInt (Variables|Default|GetCurrentWave))
      (:%20%20
        (bind _output_get (Variables|Default|SetCurrentWave _result))
        (bind _zombiesforwave (CallFunction|GetWeightforWave _output_get))
        (bind _output_get_2 (Variables|Default|SetZombieLeftInWave _zombiesforwave))
        (Variables|Default|SetWeightLeftToSpawn _output_get_2)))))

(fn ChooseZombies
  (bind _zombiweigth (Variables|Default|GetZombiWeigth))
  (while (> (Variables|Default|GetWeightLeftToSpawn) 0)
    ;[1 1 1] add zombie to zombie to spawn
    (bind _keys (Utilities|Map|Keys _zombiweigth))
    (Utilities|Array|Add (Variables|Default|GetZombiesToSpawn) (Utilities|Array|Get(acopy) _keys (Math|Random|RandomIntegerinRangefromStream 0 (stale _result) (Math|Random|MakeRandomStream (.Seconds (Class|GameplayStatics|GetAccurateRealTime))))))
    ;[1 1 1] reduce weight
    (bind _values (Utilities|Map|Values _zombiweigth))
    (Variables|Default|SetWeightLeftToSpawn (* (Utilities|Array|Get(acopy) _values (Math|Random|RandomIntegerinRangefromStream 0 (stale _result) (Math|Random|MakeRandomStream (.Seconds (Class|GameplayStatics|GetAccurateRealTime))))) -1))))