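; Vault obstacle for the parkour system that lets Player_BP perform a normal vault over it from either side.
; Right and left trigger overlaps flag the player as vault-enabled with an approach direction, and clear those flags on exit.
; On entry, a sprinting player not already vaulting starts the vault event immediately.
; IsOneWay disables entry from the left (opposite) side.
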(event OnComponentBeginOverlap(NormalVault_RightWay_Trigger)
  (params (OverlappedComponent :type Primitive%20Component%20Object%20Reference) (OtherActor :type Actor%20Object%20Reference) (OtherComp :type Primitive%20Component%20Object%20Reference) (OtherBodyIndex :type Integer) (bFromSweep :type Boolean) (SweepResult :type Hit%20Result%20Structure%20%28by%20ref%29))
  ;[1 1 1] Start normal vault from right way
  (bind _asplayer_bp (Utilities|Casting|CastToPlayer_BP OtherActor))
  (Variables|/Game/ZombieCreed_Game/Characters/Player_Character/Player_BP.Player_BP_C|SetEnableVaultParkour? _asplayer_bp true)
  (Variables|/Game/ZombieCreed_Game/Characters/Player_Character/Player_BP.Player_BP_C|SetIsRightWay? _asplayer_bp true)
  (if (and (not (Variables|/Game/ZombieCreed_Game/Characters/Player_Character/Player_BP.Player_BP_C|GetIsInNormalVaultParkour? _asplayer_bp)) (Variables|/Game/ZombieCreed_Game/Characters/Player_Character/Player_BP.Player_BP_C|GetIsSprinting _asplayer_bp))
    (Default|NormalVaultParkourEvent _asplayer_bp)))

(event OnComponentEndOverlap(NormalVault_RightWay_Trigger)
  (params (OverlappedComponent :type Primitive%20Component%20Object%20Reference) (OtherActor :type Actor%20Object%20Reference) (OtherComp :type Primitive%20Component%20Object%20Reference) (OtherBodyIndex :type Integer))
  ;[1 1 1] End normal vault on right way
  (bind _asplayer_bp (Utilities|Casting|CastToPlayer_BP OtherActor))
  (Variables|/Game/ZombieCreed_Game/Characters/Player_Character/Player_BP.Player_BP_C|SetEnableVaultParkour? _asplayer_bp false)
  (Variables|/Game/ZombieCreed_Game/Characters/Player_Character/Player_BP.Player_BP_C|SetIsRightWay? _asplayer_bp false))

(event OnComponentBeginOverlap(NormalVault_LeftWay_Trigger)
  (params (OverlappedComponent :type Primitive%20Component%20Object%20Reference) (OtherActor :type Actor%20Object%20Reference) (OtherComp :type Primitive%20Component%20Object%20Reference) (OtherBodyIndex :type Integer) (bFromSweep :type Boolean) (SweepResult :type Hit%20Result%20Structure%20%28by%20ref%29))
  ;[1 1 1] Start normal vault left way (opposite)
  (if (not (Variables|ParkourMovements|GetIsOneWay?))
    (bind _asplayer_bp (Utilities|Casting|CastToPlayer_BP OtherActor))
    (Variables|/Game/ZombieCreed_Game/Characters/Player_Character/Player_BP.Player_BP_C|SetEnableVaultParkour? _asplayer_bp true)
    (Variables|/Game/ZombieCreed_Game/Characters/Player_Character/Player_BP.Player_BP_C|SetIsOppositeWay? _asplayer_bp true)
    (if (and (not (Variables|/Game/ZombieCreed_Game/Characters/Player_Character/Player_BP.Player_BP_C|GetIsInNormalVaultParkour? _asplayer_bp)) (Variables|/Game/ZombieCreed_Game/Characters/Player_Character/Player_BP.Player_BP_C|GetIsSprinting _asplayer_bp))
      (Default|NormalVaultParkourEvent _asplayer_bp))))

(event OnComponentEndOverlap(NormalVault_LeftWay_Trigger)
  (params (OverlappedComponent :type Primitive%20Component%20Object%20Reference) (OtherActor :type Actor%20Object%20Reference) (OtherComp :type Primitive%20Component%20Object%20Reference) (OtherBodyIndex :type Integer))
  ;[1 1 1] End normal vault left way (opposite)
  (bind _asplayer_bp (Utilities|Casting|CastToPlayer_BP OtherActor))
  (Variables|/Game/ZombieCreed_Game/Characters/Player_Character/Player_BP.Player_BP_C|SetEnableVaultParkour? _asplayer_bp false)
  (Variables|/Game/ZombieCreed_Game/Characters/Player_Character/Player_BP.Player_BP_C|SetIsOppositeWay? _asplayer_bp false))

(fn ConstructionScript)